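; BP_PunchingBag is a damageable practice target that respawns after being destroyed.
; Any damage it receives passes to its health component.
; On death it hides the target cube, waits briefly, then resets health and shows the cube again.
; It also exposes its actor type through a GetActorType function.
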(event OnDeath(AC_HealthComponent)
  (Rendering|SetVisibility (Variables|Default|GetTargetCube) false false)
  (Utilities|FlowControl|Delay 1.0)
  (Default|ResetHealth (Variables|Default|GetAC_HealthComponent))
  (Rendering|SetVisibility (Variables|Default|GetTargetCube) true false))

(event Game|Damage|EventAnyDamage
  (params (Damage :type Float%20%28single-precision%29) (DamageType :type Damage%20Type%20Object%20Reference) (InstigatedBy :type Controller%20Object%20Reference) (DamageCauser :type Actor%20Object%20Reference))
  (Default|TakeDamage (Variables|Default|GetAC_HealthComponent) Damage))

(fn ConstructionScript)

(fn GetActorType
  (return (Variables|Default|GetType)))