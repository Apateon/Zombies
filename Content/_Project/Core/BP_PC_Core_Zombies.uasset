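; Player controller for the Zombies mode that requests the player's spawn and owns the HUD reference.
; On BeginPlay, the local controller calls its spawn event, which has the game mode run its spawn message for this controller.
; It then looks up the core Zombies HUD and caches it when found.
; Pressing T toggles the inventory on that cached HUD.
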(event Custom|SF_SpawnPLayer
  (Class|BIGameMode|SpawnPlayer(Message) (Game|GetGameMode) self))

(event EventBeginPlay
  (if (Pawn|IsLocalPlayerController)
    (CallFunction|SFSpawnPLayer)
    (bind _aswb_core_hud (Utilities|GetBPHCCoreZombies 0.0)
      (:Success
        (Variables|Default|SetPlayerHUD _aswb_core_hud)))))

(event Input|KeyboardEvents|T
  (params (Key :type Key%20Structure :default "None"))
  (:Pressed
    (Default|ToggleInventory (Variables|Default|GetPlayerHUD))))

(fn ConstructionScript)