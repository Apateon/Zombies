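; BP_GM_Core_Zombies is the core game mode for the Zombies game, tracking connected players and handling player spawning.
; Login and controller-swap events add Zombies player controllers to the PCs array, and logout removes them.
; SpawnPlayer destroys the controller's current pawn, spawns a BP_Player at a randomly chosen PlayerStart, and possesses it.
; Nothing in this graph calls SpawnPlayer.
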(event Custom|Add%20Player%20Controller
  (params (New%20Player%20Controller :type Player%20Controller%20Object%20Reference))
  ;[0.15 0.15 0.15 0.5] Player Connnection / Disconnection
  ;;[0.15 0.15 0.15 0.5] Adding Player to Player Controller Array
  (bind _asbp_pc_core_zombies (Utilities|Casting|CastToBP_PC_Core_Zombies New%20Player%20Controller))
  (Utilities|Array|Add (Variables|Default|GetPCs) _asbp_pc_core_zombies))

(event EventPostLogin
  (params (NewPlayer :type Player%20Controller%20Object%20Reference))
  ;[0.15 0.15 0.15 0.5] Player Connnection / Disconnection
  ;;[0.15 0.15 0.15 0.5] When Player Connects
  (CallFunction|AddPlayerController NewPlayer))

(event EventOnSwapPlayerControllers
  (params (OldPC :type Player%20Controller%20Object%20Reference) (NewPC :type Player%20Controller%20Object%20Reference))
  ;[0.15 0.15 0.15 0.5] Player Connnection / Disconnection
  ;;[0.15 0.15 0.15 0.5] When Player Connects
  (CallFunction|AddPlayerController NewPC))

(event EventOnLogout
  (params (ExitingController :type Controller%20Object%20Reference))
  ;[0.15 0.15 0.15 0.5] Player Connnection / Disconnection
  ;;[0.15 0.15 0.15 0.5] When Player Disconnects
  (bind _asbp_pc_core_zombies (Utilities|Casting|CastToBP_PC_Core_Zombies ExitingController))
  (Utilities|Array|RemoveItem (Variables|Default|GetPCs) _asbp_pc_core_zombies))

(event EventSpawnPlayer
  (params (Player%20Controller :type Player%20Controller%20Object%20Reference))
  (bind _returnvalue (Pawn|GetControlledPawn Player%20Controller))
  (Utilities|IsValid _returnvalue
    (:Is%20Valid
      (Actor|DestroyActor _returnvalue))
    (:Is%20Not%20Valid
      _))
  (bind _returnvalue_2 (Game|SpawnActorfromClass "/Game/_Project/BP_Player.BP_Player_C" (Spawning|FindRandomPlayerStart) "Undefined" "MultiplyWithRoot" 0 0))
  (Pawn|Possess Player%20Controller _returnvalue_2))

(fn ConstructionScript)

(fn FindRandomPlayerStart
  (bind _outactors (Actor|GetAllActorsOfClass "/Script/Engine.PlayerStart"))
  (return (Transformation|GetActorTransform (Utilities|Array|Get(acopy) _outactors (Math|Random|RandomIntegerinRange 0 (Utilities|Array|LastIndex _outactors))))))