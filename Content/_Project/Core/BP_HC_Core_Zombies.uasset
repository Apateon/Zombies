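; HUD Blueprint for the Zombies core that creates the player HUD and game menus and controls which menu is open.
; BeginPlay sets game-only input, adds the HUD widget to the viewport, and registers the inventory in a menu list that is also added.
; ToggleInventory calls a generic ToggleWidget, which collapses other listed menus and shows or hides the target.
; FocusWidget and FocusGame switch input mode and mouse cursor to match.
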(event Custom|Add%20Game%20Menus%20to%20Viewport
  ;[0.15 0.15 0.15 0.5] Adding Game Menus to Viewport
  (for _array_element (Variables|Default|GetGameMenu_WidgetList)
    (UserInterface|Viewport|AddtoViewport _array_element 0)))

(event Custom|ToggleInventory
  ;[0.15 0.15 0.15 0.5] Toggle Inventory
  (CallFunction|ToggleWidget (Variables|Default|GetWB_Inventory)))

(event EventBeginPlay
  (bind _returnvalue (Game|Player|GetOwningPlayerController))
  (Input|SetInputModeGameOnly _returnvalue false)
  ;[0.15 0.15 0.15 0.5] Game HUD
  (bind _returnvalue_2 (UserInterface|CreateWidget "/Game/_Project/Widgets/WB_Player_HUD.WB_Player_HUD_C" _returnvalue))
  (bind _output_get (Variables|Default|SetWB_Core_HUD _returnvalue_2))
  (UserInterface|Viewport|AddtoViewport _output_get 0)
  ;[0.15 0.15 0.15 0.5] Game Menus
  (bind _returnvalue_3 (UserInterface|CreateWidget "/Game/_Project/Widgets/WB_Inventory.WB_Inventory_C" (Game|Player|GetOwningPlayerController)))
  (bind _output_get_2 (Variables|Default|SetWB_Inventory _returnvalue_3))
  (Utilities|Array|Add (Variables|Default|GetGameMenu_WidgetList) _output_get_2)
  (CallFunction|AddGameMenustoViewport))

(fn ConstructionScript)

(fn ToggleWidget
  (params (Widget%20to%20Toggle :type User%20Widget%20Object%20Reference))
  (Utilities|IsValid Widget%20to%20Toggle
    (:Is%20Valid
      (Variables|Default|SetWidget%20to%20Focus Widget%20to%20Toggle)
      (for _array_element (Variables|Default|GetGameMenu_WidgetList)
        (Utilities|IsValid _array_element
          (:Is%20Valid
            (if (== (Variables|Default|GetWidget%20to%20Focus) _array_element)
              (if (Widget|IsVisible (Variables|Default|GetWidget%20to%20Focus))
                (CallFunction|FocusGame)
                (else
                  (CallFunction|FocusWidget)))
              (elif (Widget|IsVisible _array_element)
                (Widget|SetVisibility _array_element "Collapsed")))))))))

(fn FocusGame
  (bind _returnvalue (Game|Player|GetOwningPlayerController))
  (Widget|SetVisibility (Variables|Default|GetWidget%20to%20Focus) "Collapsed")
  (Input|SetInputModeGameOnly _returnvalue false)
  (Variables|/Script/Engine.PlayerController|SetbShowMouseCursor _returnvalue false))

(fn FocusWidget
  (bind _returnvalue (Game|Player|GetOwningPlayerController))
  (bind _widget_to_focus (Variables|Default|GetWidget%20to%20Focus))
  (Widget|SetVisibility _widget_to_focus "SelfHitTestInvisible")
  (Input|SetInputModeGameandUI _returnvalue _widget_to_focus "DoNotLock" true false)
  (Variables|/Script/Engine.PlayerController|SetbShowMouseCursor _returnvalue true))