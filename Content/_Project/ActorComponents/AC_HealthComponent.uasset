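; Actor component that tracks health for its owning actor.
; BeginPlay resets current health to the maximum.
; TakeDamage subtracts damage, fires a damage-taken event, then fires a death event once health is at or below zero, with no clamping or guard against repeat deaths.
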(event Custom|ResetHealth
  (Variables|Default|SetCurrentHealth (Variables|Default|GetMaxHealth)))

(event EventBeginPlay
  (CallFunction|ResetHealth))

(fn TakeDamage
  (params (Damage :type Float%20%28double-precision%29))
  (bind _output_get (Variables|Default|SetCurrentHealth (- (Variables|Default|GetCurrentHealth) Damage)))
  (Default|CallOnDamageTaken)
  (if (<= _output_get 0.0)
    (Default|CallOnDeath)))