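; BP_Pickup_Weapon is a world pickup that gives a weapon to the player.
; On BeginPlay it adds a hard-coded pistol component, stores it as the Weapon and copies that weapon's static mesh onto the pickup mesh.
; PickUpWeapon passes the weapon's class to the player and destroys the pickup only when the player reports success.
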(event Custom|Set%20Weapon%20Pickup
  (params (WeaponClass :type SKBP%20Master%20Weapon%20Object%20Reference))
  (bind _output_get (Variables|Default|SetWeapon WeaponClass))
  (Components|StaticMesh|SetStaticMesh (Variables|Default|GetPickupMesh) (Variables|/Game/_Project/Props/Weapons/SKBP_MasterWeapon.SKBP_MasterWeapon_C|GetStaticMesh _output_get)))

(event EventPickUpWeapon
  (params (PickUpPlayer :type BP%20Player%20Object%20Reference))
  (bind _pickupsuccess (Default|PickUpWeapon PickUpPlayer (Utilities|GetClass (Variables|Default|GetWeapon))))
  (if _pickupsuccess
    (Actor|DestroyActor)))

(event EventBeginPlay
  (bind _returnvalue (Game|AddComponentbyClass "/Game/_Project/Props/Weapons/SKBP_Weapon_Pistol.SKBP_Weapon_Pistol_C" false))
  (CallFunction|SetWeaponPickup _returnvalue))

(fn ConstructionScript
  (|CallParentFunction))