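; Base enemy Blueprint that tracks health and respawns in place shortly after dying.
; Any incoming damage goes through TakeDamage, which clamps health and, at zero, hides the mesh and clears IsAlive.
; After a short delay, Respawn restores full health, visibility and the alive flag on the same actor.
; Death only toggles mesh visibility; collision is untouched and the actor is never destroyed.
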(event EventBeginPlay
  (Variables|Default|SetCurrentHealth (Variables|Default|GetMaxHealth)))

(event Game|Damage|EventAnyDamage
  (params (Damage :type Float%20%28single-precision%29) (DamageType :type Damage%20Type%20Object%20Reference) (InstigatedBy :type Controller%20Object%20Reference) (DamageCauser :type Actor%20Object%20Reference))
  (CallFunction|TakeDamage Damage)
  (if (not (Variables|Default|GetIsAlive))
    (Utilities|FlowControl|Delay 1.0)
    (CallFunction|Respawn)))

(fn ConstructionScript)

(fn TakeDamage
  (params (Damage :type Float%20%28double-precision%29))
  (bind _output_get (Variables|Default|SetCurrentHealth (Math|Float|Clamp(Float) (- (Variables|Default|GetCurrentHealth) Damage) 0.0 (Variables|Default|GetMaxHealth))))
  (if (== _output_get 0.0)
    (Rendering|SetVisibility (Variables|Character|GetMesh) false false)
    (Variables|Default|SetIsAlive false)))

(fn Respawn
  (Variables|Default|SetCurrentHealth (Variables|Default|GetMaxHealth))
  (Rendering|SetVisibility (Variables|Character|GetMesh) true false)
  (Variables|Default|SetIsAlive true))