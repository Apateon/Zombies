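; Base magnetic pickup that flies to the player and delivers a typed refill amount, with item and ammo types set on BeginPlay.
; Range overlap asks the overlapping actor via message whether it requires the item; if so, it stores that actor as target.
; A timeline then moves the pickup by interpolating toward player character 0 plus a track offset.
; When the mesh overlaps the target, it sends the refill message and destroys itself.
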(event OnComponentBeginOverlap(ItemMesh)
  (params (OverlappedComponent :type Primitive%20Component%20Object%20Reference) (OtherActor :type Actor%20Object%20Reference) (OtherComp :type Primitive%20Component%20Object%20Reference) (OtherBodyIndex :type Integer) (bFromSweep :type Boolean) (SweepResult :type Hit%20Result%20Structure%20%28by%20ref%29))
  (if (and (== OtherActor (Variables|Default|GetTarget)) (Variables|Default|GetRequired))
    (Class|BPIItemPicker|TakeRefill(Message) OtherActor (Variables|Default|GetRefillAmount) (Variables|Default|GetItemType) (Variables|Default|GetAmmoType))
    (Actor|DestroyActor)))

(event OnComponentBeginOverlap(PickupRange)
  (params (OverlappedComponent :type Primitive%20Component%20Object%20Reference) (OtherActor :type Actor%20Object%20Reference) (OtherComp :type Primitive%20Component%20Object%20Reference) (OtherBodyIndex :type Integer) (bFromSweep :type Boolean) (SweepResult :type Hit%20Result%20Structure%20%28by%20ref%29))
  (bind _need (Class|BPIItemPicker|RequireAttractable(Message) OtherActor (Variables|Default|GetItemType) (Variables|Default|GetAmmoType)))
  (if _need
    (Variables|Default|SetRequired _need)
    (Variables|Default|SetTarget OtherActor)
    (bind _newtrack_0 (Timeline|Timeline PlayFromStart)
      (:Update
        (Transformation|SetActorLocation (+ _newtrack_0 (Math|Interpolation|VInterpTo (.Location (Math|Transform|BreakTransform (Transformation|GetActorTransform))) (Transformation|GetActorLocation (Game|GetPlayerCharacter 0)) (Utilities|Time|GetWorldDeltaSeconds) 1e+01)) false false)))))

(event EventBeginPlay
  (Variables|Default|SetItemType "NewEnumerator1")
  (Variables|Default|SetAmmoType "NewEnumerator1")
  (Variables|Default|SetRefillAmount 1e+01))

(fn ConstructionScript)