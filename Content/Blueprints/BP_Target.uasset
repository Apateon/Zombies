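; BP_Target is a damageable target actor that hides when its health runs out and respawns shortly afterwards.
; AnyDamage feeds TakeDamage, which clamps Health and, at zero, hides TargetCube and clears IsAlive.
; After a brief delay, Respawn restores full health and visibility on the same actor.
; It also prints a greeting on Interact and reports its Type through GetActorType.
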(event EventBeginPlay
  (Variables|Default|SetHealth (Variables|Default|GetMaxHealth)))

(event Game|Damage|EventAnyDamage
  (params (Damage :type Float%20%28single-precision%29) (DamageType :type Damage%20Type%20Object%20Reference) (InstigatedBy :type Controller%20Object%20Reference) (DamageCauser :type Actor%20Object%20Reference))
  (CallFunction|TakeDamage Damage)
  (if (not (Variables|Default|GetIsAlive))
    (Utilities|FlowControl|Delay 1.0)
    (CallFunction|Respawn)))

(event EventInteract
  (params (Interactor :type Actor%20Object%20Reference))
  (Development|PrintString "Hello"))

(fn ConstructionScript)

(fn Respawn
  (Variables|Default|SetHealth (Variables|Default|GetMaxHealth))
  (Rendering|SetVisibility (Variables|Default|GetTargetCube) true false)
  (Variables|Default|SetIsAlive true))

(fn TakeDamage
  (params (Damage :type Float%20%28double-precision%29))
  (bind _output_get (Variables|Default|SetHealth (Math|Float|Clamp(Float) (- (Variables|Default|GetHealth) Damage) 0.0 (Variables|Default|GetMaxHealth))))
  (if (== _output_get 0.0)
    (Rendering|SetVisibility (Variables|Default|GetTargetCube) false false)
    (Variables|Default|SetIsAlive false)))

(fn GetActorType
  (return (Variables|Default|GetType)))