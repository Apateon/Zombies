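; Pistol weapon Blueprint that implements the primary fire as an instant hitscan shot.
; WeaponPrimary line traces on the Visibility channel between the supplied start and end locations.
; On a hit, it attaches a bullet hole to the hit component, aligned to the surface normal, and calls DealDamage on the hit actor with the Damage value and shooter.
; The event graph holds no active logic.
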(event EventBeginPlay
  (|CallParentFunction) ; This node is disabled and will not be called.\nDrag off pins to build functionality.
)

(event Collision|EventActorBeginOverlap
  (params (OtherActor :type Actor%20Object%20Reference)))

(event EventTick
  (params (DeltaSeconds :type Float%20%28single-precision%29)))

(fn ConstructionScript
  (|CallParentFunction))

(fn WeaponPrimary
  (params (Start%20Location :type Vector :default "0, 0, 0") (End%20Location :type Vector :default "0, 0, 0") (Shooter :type E_ActorType%20Enum :default "NewEnumerator1"))
  (bind (_outhit _returnvalue) (Collision|LineTraceByChannel Start%20Location End%20Location "TraceTypeQuery1" false 0 "None" true "(R=1.000000,G=0.000000,B=0.000000,A=1.000000)" "(R=0.000000,G=1.000000,B=0.000000,A=1.000000)" 3.0))
  (if _returnvalue
    (CallFunction|MakeBulletHole (.HitComponent (Collision|BreakHitResult _outhit)) (.Location (Collision|BreakHitResult _outhit)) (Math|Conversions|RotationFromXVector (.Normal (Collision|BreakHitResult _outhit))))
    (CallFunction|DealDamage (.HitActor (Collision|BreakHitResult _outhit)) (Variables|Default|GetDamage) Shooter)))