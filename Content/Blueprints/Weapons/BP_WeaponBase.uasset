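; Base weapon Blueprint that tracks magazine and reserve ammo and provides shared damage and pickup logic.
; BeginPlay fills the magazine and reads reserve limits by ammo type, while Reload and AddAmmo update the counts within those limits.
; DealDamage skips targets whose actor type matches the shooter's, and Interact destroys the actor.
; WeaponPrimary is an empty firing hook, presumably for child weapons to override.
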(event EventBeginPlay
  (Variables|Default|SetCurrentAmmo (Variables|Default|GetMaxAmmo))
  (bind (_reserveammo _maxreserve) (CallFunction|GetAmmoReserve (Variables|Default|GetAmmoType)))
  (Variables|Default|SetAmmoReserve _reserveammo)
  (Variables|Default|SetMaxReserve _maxreserve))

(event EventInteract
  (params (Interactor :type Actor%20Object%20Reference))
  (Actor|DestroyActor))

(fn ConstructionScript)

(fn GetMesh
  (return (Variables|/Script/Engine.StaticMeshComponent|GetStaticMesh (Variables|Default|GetGunMesh))))

(fn Reload
  (Variables|Default|SetAmmoReserve (- (Variables|Default|GetAmmoReserve) (Math|Integer|Clamp(Integer) (- (Variables|Default|GetMaxAmmo) (Variables|Default|GetCurrentAmmo)) 0 (Variables|Default|GetAmmoReserve))))
  (Variables|Default|SetCurrentAmmo (+ (Math|Integer|Clamp(Integer) (- (Variables|Default|GetMaxAmmo) (Variables|Default|GetCurrentAmmo)) 0 (Variables|Default|GetAmmoReserve)) (Variables|Default|GetCurrentAmmo))))

(fn DealDamage
  (params (HitActor :type Actor%20Object%20Reference) (Damage :type Float%20%28double-precision%29) (Shooter :type E_ActorType%20Enum :default "NewEnumerator1"))
  (bind _actortype (Class|BPIDamagable|GetActorType(Message) HitActor))
  (if (Utilities|Enum|NotEqual(Enum) _actortype Shooter)
    (Game|Damage|ApplyDamage HitActor Damage 0 0)))

(fn NeedAmmo?
  (params (AmmoType :type E_AmmoType%20Enum :default "NewEnumerator3"))
  (return (and (Utilities|Enum|Equal(Enum) AmmoType (Variables|Default|GetAmmoType)) (< (Variables|Default|GetAmmoReserve) (Variables|Default|GetMaxReserve)))))

(fn AddAmmo
  (params (Ammo :type Float%20%28double-precision%29))
  (Variables|Default|SetAmmoReserve (Math|Float|Truncate (Math|Float|Min(Float) (+ Ammo (Variables|Default|GetAmmoReserve)) (Math|Conversions|ToFloat(Integer) (Variables|Default|GetMaxReserve))))))

(fn WeaponPrimary
  (params (Start%20Location :type Vector) (End%20Location :type Vector) (Shooter :type E_ActorType%20Enum :default "NewEnumerator1")))