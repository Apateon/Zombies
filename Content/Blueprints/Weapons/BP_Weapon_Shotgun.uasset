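; Shotgun weapon Blueprint whose primary fire shoots several hitscan pellets at once.
; WeaponPrimary loops line traces on the Visibility channel, offsetting each trace's end point by a random Spread value on every axis.
; Each hit attaches a bullet hole aligned to the surface normal and deals Damage to the hit actor, crediting the Shooter.
; The construction script only calls its parent.
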(fn ConstructionScript
  (|CallParentFunction))

(fn WeaponPrimary
  (params (Start%20Location :type Vector :default "0, 0, 0") (End%20Location :type Vector :default "0, 0, 0") (Shooter :type E_ActorType%20Enum :default "NewEnumerator1"))
  (for _index (range 0 3)
    (bind _randomspread (CallFunction|RandomSpread (Variables|Default|GetSpread)))
    (bind _randomspread_2 (CallFunction|RandomSpread (Variables|Default|GetSpread)))
    (bind _randomspread_3 (CallFunction|RandomSpread (Variables|Default|GetSpread)))
    (bind (_outhit _returnvalue) (Collision|LineTraceByChannel Start%20Location (+ End%20Location (Math|Vector|MakeVector _randomspread _randomspread_2 _randomspread_3)) "TraceTypeQuery1" false 0 "None"))
    (if _returnvalue
      (CallFunction|MakeBulletHole (.HitComponent (Collision|BreakHitResult _outhit)) (.Location (Collision|BreakHitResult _outhit)) (Math|Conversions|RotationFromXVector (.Normal (Collision|BreakHitResult _outhit))))
      (CallFunction|DealDamage (.HitActor (Collision|BreakHitResult _outhit)) (Variables|Default|GetDamage) Shooter))))