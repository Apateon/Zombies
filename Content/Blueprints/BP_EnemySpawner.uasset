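; Enemy spawner actor that runs round-based waves of BP_Enemy_Scrapper.
; CreateEnemies loops with a delay, spawning at random reachable navmesh points around the spawner until the round's total is reached, and passes each enemy a spawner reference.
; EnemyKilled decrements the live count; at zero it advances the round, scales the total linearly, shortens the delay exponentially to a minimum, and restarts spawning.
; BeginPlay is empty.
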(event Custom|Create%20Enemies
  ;[0.15 0.15 0.15 0.5] Enemy Loop
  (if (> (Variables|Default|GetTotalEnemies) (Variables|Default|GetCurrentEnemies)) :!label _label
    (Utilities|FlowControl|Delay (Variables|Default|GetSpawnSpeed))
    (Math|Integer|IncrementInt (Variables|Default|GetCurrentEnemies)
      (:%20%20
        (bind _returnvalue (Game|SpawnActorfromClass "/Game/Blueprints/Characters/Enemies/BP_Enemy_Scrapper.BP_Enemy_Scrapper_C" (Math|Transform|MakeTransform (.RandomLocation (AI|Navigation|GetRandomReachablePointinRadius (Transformation|GetActorLocation) 7e+03 0 0)) "0, 0, 0" "1.000000,1.000000,1.000000") "Undefined" "MultiplyWithRoot" 0 0))
        (Default|GetSpawner _returnvalue self)
        (goto _label)))))

(event EventBeginPlay)

(event EventEnemyKilled
  (bind _result (Math|Integer|DecrementInt (Variables|Default|GetCurrentEnemies))
    (:%20%20
      (if (<= _result 0)
        (bind _result_2 (Math|Integer|IncrementInt (Variables|Default|GetRoundNumber))
          (:%20%20
            (Variables|Default|SetTotalEnemies (* _result_2 5))
            (Variables|Default|SetSpawnSpeed (Math|Float|Max(Float) (* 2.0 (Math|Float|Power 0.95 (Math|Conversions|ToFloat(Integer) (- (Variables|Default|GetRoundNumber) 1)))) 0.1))
            (CallFunction|CreateEnemies)))))))

(fn ConstructionScript)