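; BP_BaseCharacter is a base character Blueprint that holds health, alive state and an actor type.
; TakeDamage subtracts damage from CurrentHealth, clamps it between zero and MaxHealth, and clears IsAlive when health reaches zero.
; GetActorType returns the stored ActorType, and the construction script is empty.
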(fn ConstructionScript)

(fn TakeDamage
  (params (Damage :type Float%20%28double-precision%29))
  (bind _output_get (Variables|Default|SetCurrentHealth (Math|Float|Clamp(Float) (- (Variables|Default|GetCurrentHealth) Damage) 0.0 (Variables|Default|GetMaxHealth))))
  (Variables|Default|SetIsAlive (not (== _output_get 0.0)))
  (return))

(fn GetActorType
  (return (Variables|Default|GetActorType)))