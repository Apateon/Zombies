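; Base enemy Blueprint that handles health, damage and death, and notifies its spawner when killed.
; BeginPlay fills health to max, and AnyDamage routes into a TakeDamage override that calls the parent and hides the mesh on death.
; Once no longer alive, the enemy messages its Spawner reference and destroys itself.
; Attack is an empty stub, and GetSpawner exposes the spawner reference.
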(event EventBeginPlay
  (Variables|Default|SetCurrentHealth (Variables|Default|GetMaxHealth)))

(event Game|Damage|EventAnyDamage
  (params (Damage :type Float%20%28single-precision%29) (DamageType :type Damage%20Type%20Object%20Reference) (InstigatedBy :type Controller%20Object%20Reference) (DamageCauser :type Actor%20Object%20Reference))
  (CallFunction|TakeDamage Damage)
  (if (not (Variables|Default|GetIsAlive))
    (Class|BPIEnemySpawner|EnemyKilled(Message) (Variables|Default|GetSpawner))
    (Actor|DestroyActor)))

(fn ConstructionScript)

(fn Attack)

(fn TakeDamage
  (params (Damage :type Float%20%28double-precision%29))
  (|CallParentFunction Damage)
  (if (not (Variables|Default|GetIsAlive))
    (Rendering|SetVisibility (Variables|Character|GetMesh) false false)))

(fn GetSpawner
  (params (Spawner :type Actor%20Object%20Reference))
  (Variables|Default|SetSpawner Spawner))