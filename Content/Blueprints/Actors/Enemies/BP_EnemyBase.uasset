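; Base enemy actor Blueprint that takes damage, disappears on death and respawns after a short delay.
; AnyDamage feeds a TakeDamage override, which calls the parent implementation and hides the mesh when IsAlive is false.
; The event then waits before Respawn restores full health, mesh visibility and the alive flag.
; Attack and the construction script are empty.
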(event Game|Damage|EventAnyDamage
  (params (Damage :type Float%20%28single-precision%29) (DamageType :type Damage%20Type%20Object%20Reference) (InstigatedBy :type Controller%20Object%20Reference) (DamageCauser :type Actor%20Object%20Reference))
  (CallFunction|TakeDamage Damage)
  (if (not (Variables|Default|GetIsAlive))
    (Utilities|FlowControl|Delay 1.0)
    (CallFunction|Respawn)))

(fn ConstructionScript)

(fn Respawn
  (Variables|Default|SetCurrentHealth (Variables|Default|GetMaxHealth))
  (Rendering|SetVisibility (Variables|Character|GetMesh) true false)
  (Variables|Default|SetIsAlive true))

(fn Attack)

(fn TakeDamage
  (params (Damage :type Float%20%28double-precision%29))
  (|CallParentFunction Damage)
  (if (not (Variables|Default|GetIsAlive))
    (Rendering|SetVisibility (Variables|Character|GetMesh) false false)))