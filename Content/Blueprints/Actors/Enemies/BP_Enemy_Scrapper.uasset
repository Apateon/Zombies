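; BP_Enemy_Scrapper is an enemy actor with a short-range melee-style attack.
; EnemyAttack fires a visibility line trace 55 units forward from AttackOrigin and applies fixed damage to the hit actor if its type differs from the Scrapper's ActorType.
; Type lookup uses a GetActorType message, which the Scrapper also implements to return its own enum value.
; The construction script only calls its parent's.
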(event EventEnemyAttack
  (bind _attackorigin (Variables|Default|GetAttackOrigin))
  (bind _returnvalue (Transformation|GetWorldLocation _attackorigin))
  (bind (_outhit _returnvalue_2) (Collision|LineTraceByChannel _returnvalue (+ _returnvalue (* (Math|Vector|GetForwardVector _attackorigin) 55.0)) "TraceTypeQuery1" false 0 "None"))
  (if _returnvalue_2
    (bind _actortype (Class|BPIDamagable|GetActorType(Message) (.HitActor (Collision|BreakHitResult _outhit))))
    (if (Utilities|Enum|NotEqual(Enum) _actortype (Variables|Default|GetActorType))
      (Game|Damage|ApplyDamage (.HitActor (Collision|BreakHitResult _outhit)) 1e+01 0 0))))

(fn ConstructionScript
  (|CallParentFunction))

(fn GetActorType
  (return "NewEnumerator1"))